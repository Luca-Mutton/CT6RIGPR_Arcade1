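; Game mode for an arcade ball game that tracks score, lives and an elapsed minutes-and-seconds timer driven by a delayed Tick.
; The ball's OnDestroyed event spawns and possesses a replacement, decrements lives and rebinds itself.
; When lives run out, it inserts the score under a hard-coded name into the saved ranking using a DoOnce, saves, then pauses on a scoreboard widget.
; Separate functions add or subtract points in fixed steps.
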(event `self.ReceiveTick`
  (params (DeltaSeconds :type "Float (single-precision)"))
  ;[0.1073 1 0.2812] Timer for level
  (`KismetSystemLibrary.Delay` 1.0) ; Timer ticks down every second
  (set `self.Seconds` (+ (`self.Seconds`) 1))
  (if (>= (`self.Seconds`) 60)
    (set `self.Minutes` (+ (`self.Minutes`) 1)) ; set minute
    (set `self.Seconds` 0) ; reset seconds back to 0
  ))

(event `RespawnPlayer`
  (params (DestroyedActor :type "Actor Object Reference"))
  ;[1 1 1] Respawn Player (take away a life)
  (bind _result (`/Engine/EditorBlueprintResources/StandardMacros.DecrementInt` (`self.Lives`))
    (:`  `
      (set `self.Lives` _result)
      ;[1 1 1] Respawn player
      (bind _asbp_ct6rigpr_arcade_1ball (cast `/Game/Blueprints/BP_CT6RIGPR_Arcade1Ball` (`GameplayStatics.GetPlayerPawn` 0) :!label _label))
      (add `self.OnDestroyed` _asbp_ct6rigpr_arcade_1ball (delegate `OnDestroyevent`)))))

(event `self.ReceiveBeginPlay`
  (goto _label))

(event `OnDestroyevent` :!signature `self.OnDestroyed`
  (params (DestroyedActor :type "Actor Object Reference"))
  (bind _returnvalue (`GameplayStatics.GetPlayerController` 0))
  (bind _temp (`self.Temp`))
  (bind _score (`self.Score`))
  ;[1 1 1] Respawn player
  (bind _returnvalue_2 (`|SpawnActorFromClass` "/Game/Blueprints/BP_CT6RIGPR_Arcade1Ball.BP_CT6RIGPR_Arcade1Ball_C" (`self.SpawnLocation`) "Undefined" "OverrideRootScale" null null))
  (`Controller.Possess` (`GameplayStatics.GetPlayerController` 0) _returnvalue_2)
  (`self.RespawnPlayer` null)
  (if (<= (`self.Lives`) 0)
    (`/Engine/EditorBlueprintResources/StandardMacros.DoOnce` false
      (:`Completed`
        ;[1 0.2973 0] Setting Highscore
        (bind _returnvalue_3 (`GameplayStatics.LoadGameFromSlot` "BP_SaveScore")) ; load the contents from a given slot
        (bind _asbp_save_score (cast `/Game/Blueprints/GameplayElements/Score_System/BP_SaveScore` _returnvalue_3)
          (:`then`
            (for _array_element (`/Game/Blueprints/GameplayElements/Score_System/BP_SaveScore.PlayerScore` _asbp_save_score)
              (`|ExecutionSequence`
                (:`then_0`
                  (if (<= (`.Score_14_BDD3F1424C08A3C1360EDF8331D0F0D8` (break `/Game/Blueprints/GameplayElements/Score_System/Score` _array_element)) _score)
                    (`/Engine/EditorBlueprintResources/StandardMacros.DoOnce` false :!label _label_2
                      (:`Completed`
                        (`KismetArrayLibrary.Array_Add` _temp (make `/Game/Blueprints/GameplayElements/Score_System/Score` "Luca" _score (`KismetMathLibrary.GetDate` (struct))))))))
                (:`then_1`
                  (`KismetArrayLibrary.Array_Add` _temp _array_element))))
            (`|ExecutionSequence`
              (:`then_0`
                (goto _label_2))
              (:`then_1`
                (bind _returnvalue_4 (`GameplayStatics.CreateSaveGameObject` "/Game/Blueprints/GameplayElements/Score_System/BP_SaveScore.BP_SaveScore_C" :!label _label_3)) ; create a new save game object
                (bind _asbp_save_score_2 (cast `/Game/Blueprints/GameplayElements/Score_System/BP_SaveScore` _returnvalue_4))
                (set `/Game/Blueprints/GameplayElements/Score_System/BP_SaveScore.PlayerScore` _temp _asbp_save_score_2)
                (`GameplayStatics.SaveGameToSlot` _returnvalue_4 "BP_SaveScore") ; save game into specfici slot/file
                (bind _returnvalue_5 (`|CreateWidget` "/Game/Blueprints/GameplayElements/UI/BP_Scoreboard.BP_Scoreboard_C" null _temp))
                (`UserWidget.AddToViewport` _returnvalue_5 0)
                (`WidgetBlueprintLibrary.SetInputMode_UIOnlyEx` _returnvalue (`/Game/Blueprints/GameplayElements/UI/BP_Scoreboard.Retry` _returnvalue_5))
                (set `PlayerController.bShowMouseCursor` true _returnvalue)
                (`GameplayStatics.SetGamePaused` true))))
          (:`CastFailed`
            (`|ExecutionSequence`
              (:`then_0`
                (goto _label_2))
              (:`then_1`
                (goto _label_3)))))))))

(event `TileRespawn`
  (params (DestroyedActor :type "Actor Object Reference")))

(fn `Add points`
  (set `self.Score` (+ (`self.Score`) 100)))

(fn `Minus Points`
  (if (<= (`self.Score`) 0)
    (set `self.Score` 0)
    (else
      (set `self.Score` (- (`self.Score`) 100)))))

(fn `UserConstructionScript`)