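; BP_FinishGame is a finish trigger actor that ends the game once the player's ball reaches it with enough points.
; On box overlap by BP_CT6RIGPR_Arcade1Ball, it compares the game mode's Score with TotalPointsRequired.
; If the score suffices, it calls the game mode's Scoreboard once; otherwise it prints a not-enough-points message.
; Disconnected leftover nodes for scoreboard widgets, pausing and high-score saving never run.
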(event `self.Box.OnComponentBeginOverlap`
  (params (OverlappedComponent :type "PrimitiveComponent Object Reference") (OtherActor :type "Actor Object Reference") (OtherComp :type "PrimitiveComponent Object Reference") (OtherBodyIndex :type Integer) (bFromSweep :type Boolean) (SweepResult :type "HitResult Structure (by ref)"))
  (cast `/Game/Blueprints/BP_CT6RIGPR_Arcade1Ball` OtherActor)
  (bind _asmy_ct6rigpr_arcade_1game_mode (cast `/Game/Blueprints/MyCT6RIGPR_Arcade1GameMode` (`GameplayStatics.GetGameMode`)))
  (if (>= (`/Game/Blueprints/MyCT6RIGPR_Arcade1GameMode.Score` _asmy_ct6rigpr_arcade_1game_mode) (`self.TotalPointsRequired`))
    (`/Engine/EditorBlueprintResources/StandardMacros.DoOnce` false
      (:`Completed`
        (bind _asmy_ct6rigpr_arcade_1game_mode_2 (cast `/Game/Blueprints/MyCT6RIGPR_Arcade1GameMode` (`GameplayStatics.GetGameMode`)))
        (`/Game/Blueprints/MyCT6RIGPR_Arcade1GameMode.Scoreboard` _asmy_ct6rigpr_arcade_1game_mode_2)))
    (else
      (`KismetSystemLibrary.PrintString` "Not enough points"))))

(fn `UserConstructionScript`)