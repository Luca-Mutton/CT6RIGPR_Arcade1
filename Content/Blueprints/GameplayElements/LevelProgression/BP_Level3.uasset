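; BP_Level3 is a level progression trigger that gates the exit to the next level on the player's score.
; When the arcade ball overlaps its box, it compares the game mode's Score against TotalPointsRequired.
; With enough points, it shows the BP_Level3 widget focused on NextLevel, enables the mouse cursor and pauses the game.
; Otherwise it only prints a not-enough-points message.
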(event `self.Box.OnComponentBeginOverlap`
  (params (OverlappedComponent :type "PrimitiveComponent Object Reference") (OtherActor :type "Actor Object Reference") (OtherComp :type "PrimitiveComponent Object Reference") (OtherBodyIndex :type Integer) (bFromSweep :type Boolean) (SweepResult :type "HitResult Structure (by ref)"))
  (bind _returnvalue (`GameplayStatics.GetPlayerController` 0))
  (cast `/Game/Blueprints/BP_CT6RIGPR_Arcade1Ball` OtherActor)
  (bind _asmy_ct6rigpr_arcade_1game_mode (cast `/Game/Blueprints/MyCT6RIGPR_Arcade1GameMode` (`GameplayStatics.GetGameMode`)))
  (if (>= (`/Game/Blueprints/MyCT6RIGPR_Arcade1GameMode.Score` _asmy_ct6rigpr_arcade_1game_mode) (`self.TotalPointsRequired`))
    (bind _returnvalue_2 (`|CreateWidget` "/Game/Blueprints/GameplayElements/UI/BP_Level3.BP_Level3_C"))
    (`UserWidget.AddToViewport` _returnvalue_2 0)
    (`WidgetBlueprintLibrary.SetInputMode_GameAndUIEx` _returnvalue (`/Game/Blueprints/GameplayElements/UI/BP_Level3.NextLevel` _returnvalue_2))
    (set `PlayerController.bShowMouseCursor` true _returnvalue)
    (`GameplayStatics.SetGamePaused` true)
    (else
      (`KismetSystemLibrary.PrintString` "Not enough points"))))

(fn `UserConstructionScript`)