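; BP_Platform1 is a falling platform obstacle that drops away under the player's arcade ball.
; Overlap events on its Box respond only to the ball, and the Timed flag selects the trigger.
; Timed platforms swap the Hex mesh material on contact and fall after Time seconds, while untimed ones fall shortly after the ball leaves.
; Both paths share one sequence that enables physics on Hex, then destroys the actor after a delay.
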(event `self.Box.OnComponentBeginOverlap`
  (params (OverlappedComponent :type "PrimitiveComponent Object Reference") (OtherActor :type "Actor Object Reference") (OtherComp :type "PrimitiveComponent Object Reference") (OtherBodyIndex :type Integer) (bFromSweep :type Boolean) (SweepResult :type "HitResult Structure (by ref)"))
  (bind _hex (`self.Hex`))
  ;[1 1 1] Overlap event for falling platform
  (cast `/Game/Blueprints/BP_CT6RIGPR_Arcade1Ball` OtherActor)
  (if (`self.Timed`)
    (`PrimitiveComponent.SetMaterial` _hex 1 "/Game/Blueprints/GameplayElements/Obstacles/PlatformColour2.PlatformColour2")
    (`KismetSystemLibrary.Delay` (`self.Time`))
    (`PrimitiveComponent.SetSimulatePhysics` _hex true :!label _label) ; Targets cube to fall when the player is on top of collision box
    (`KismetSystemLibrary.Delay` 4.0) ; Sets a delay for object to disappear
    (`self.K2_DestroyActor`) ; Destroys object
  ))

(event `self.Box.OnComponentEndOverlap`
  (params (OverlappedComponent :type "PrimitiveComponent Object Reference") (OtherActor :type "Actor Object Reference") (OtherComp :type "PrimitiveComponent Object Reference") (OtherBodyIndex :type Integer))
  ;[1 1 1] Overlap event for falling platform
  (cast `/Game/Blueprints/BP_CT6RIGPR_Arcade1Ball` OtherActor)
  (if (not (`self.Timed`))
    (`KismetSystemLibrary.Delay` 0.2)
    (goto _label)))

(fn `UserConstructionScript`)