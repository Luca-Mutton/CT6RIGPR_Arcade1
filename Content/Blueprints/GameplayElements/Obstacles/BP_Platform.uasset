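; Hex platform obstacle that drops when the arcade ball character touches or leaves it, depending on the Timed flag.
; When timed, entering the box turns the hex red and starts the fall after a delay; otherwise leaving the box triggers it.
; The MoveVertical timeline lerps the hex down from its BeginPlay location.
; Delays chained off the timeline update hide the actor and disable collision, then restore both with blue material.
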(event `self.ReceiveBeginPlay`
  (set `self.StartPoint` (`self.K2_GetActorLocation`)))

(event `self.Box.OnComponentBeginOverlap`
  (params (OverlappedComponent :type "PrimitiveComponent Object Reference") (OtherActor :type "Actor Object Reference") (OtherComp :type "PrimitiveComponent Object Reference") (OtherBodyIndex :type Integer) (bFromSweep :type Boolean) (SweepResult :type "HitResult Structure (by ref)"))
  ;[1 1 1] Overlap event for falling platform
  (cast `/Game/Blueprints/BP_CT6RIGPR_Arcade1Ball` OtherActor) ; cast to character
  (if (`self.Timed`)
    (`PrimitiveComponent.SetMaterial` (`self.Hex`) 0 "/Game/ExperimentVisuals/floor-TileMat/Red.Red") ; change the material of mesh
    (`KismetSystemLibrary.Delay` (`self.Time`)) ; start countdown for object to fall
    (bind (_direction _movevertical) (`Timeline|MoveVertical` :!via `PlayFromStart` :!label _label)
      (:`Update`
        (`SceneComponent.K2_SetWorldLocation` (`self.Hex`) (`KismetMathLibrary.VLerp` (`self.StartPoint`) (- (`self.StartPoint`) (`self.EndPoint`)) _movevertical) false false)
        (`KismetSystemLibrary.Delay` 3.0)
        (`self.SetActorHiddenInGame` true) ; hides an actor
        (`self.SetActorEnableCollision` false) ; delete collision when hidden
        (`KismetSystemLibrary.Delay` 5.0)
        (`self.SetActorHiddenInGame` false)
        (`PrimitiveComponent.SetMaterial` (`self.Hex`) 0 "/Game/ExperimentVisuals/floor-TileMat/Blue.Blue")
        (`self.SetActorEnableCollision` true)))))

(event `self.Box.OnComponentEndOverlap`
  (params (OverlappedComponent :type "PrimitiveComponent Object Reference") (OtherActor :type "Actor Object Reference") (OtherComp :type "PrimitiveComponent Object Reference") (OtherBodyIndex :type Integer))
  ;[1 1 1] Overlap event for falling platform
  (cast `/Game/Blueprints/BP_CT6RIGPR_Arcade1Ball` OtherActor) ; Cast to character
  (if (not (`self.Timed`))
    (goto _label :!via `PlayFromStart`)))

(fn `UserConstructionScript`)