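; Player-controlled arcade ball that rolls through a level while tracking score and elapsed time.
; Move inputs apply torque to the ball along the camera's axes, and turn inputs drive controller yaw.
; A Delay on Tick counts seconds up into minutes; the countdown and game-over widget logic is left disconnected.
; Functions add or subtract points in fixed steps and add a minute to the timer.
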(event `InputAxis|TurnRate`
  (params (AxisValue :type "Float (single-precision)"))
  ;[1 1 1] Turn rate of camera
  (`self.AddControllerYawInput` (* AxisValue (`self.BaseTurnRate`) (`GameplayStatics.GetWorldDeltaSeconds`))))

(event `InputAxis|MoveForward` :overrideparent false
  (params (AxisValue :type "Float (single-precision)"))
  ;[1 1 1] Movement in world direction
  (`PrimitiveComponent.AddTorqueInRadians` (`self.Ball`) (* (`SceneComponent.GetRightVector` (`self.Camera`)) (* AxisValue (`self.Roll Torque`))) "None" false))

(event `InputAxis|Turn`
  (params (AxisValue :type "Float (single-precision)"))
  ;[1 1 1] Turn direction of camera
  (`self.AddControllerYawInput` AxisValue))

(event `InputAxis|MoveRight` :overrideparent false
  (params (AxisValue :type "Float (single-precision)"))
  ;[1 1 1] Movement in world direction
  (`PrimitiveComponent.AddTorqueInRadians` (`self.Ball`) (* (* (`SceneComponent.GetForwardVector` (`self.Camera`)) (* AxisValue (`self.Roll Torque`))) -1.0) "None" false))

(event `self.ReceiveBeginPlay`)

(event `self.ReceiveTick`
  (params (DeltaSeconds :type "Float (single-precision)"))
  ;[0.1073 1 0.2812] Timer for level
  (`KismetSystemLibrary.Delay` 1.0) ; Timer ticks down every second
  (set `self.Seconds` (+ (`self.Seconds`) 1))
  (if (>= (`self.Seconds`) 60)
    (set `self.Minutes` (+ (`self.Minutes`) 1)) ; set minute
    (set `self.Seconds` 0) ; reset seconds back to 0
  ))

(fn `Add points`
  ;[1 1 1] Add points from coin objects
  (set `self.Score` (+ (`self.Score`) 100)) ; Sets score
)

(fn `Minus Points`
  ;[1 0.9123 0.1124] Minus points fucntion
  (if (<= (`self.Score`) 0)
    (set `self.Score` 0)
    (else
      (set `self.Score` (- (`self.Score`) 100)) ; Sets score
    )))

(fn `Time Increase`
  (set `self.Minutes` (+ 1 (`self.Minutes`))))

(fn `UserConstructionScript`)